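; A collectible coin pickup for a paper-sprite player, worth a common low value or, on a random roll at BeginPlay, a rarer high value tinted green.
; On overlap with the player it adds its value to the player's ScoreSystem and destroys itself.
; Tick watches the player's sweet-spot combo, doubling the value and swapping the sprite above a threshold, then restoring both when the combo drops.
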(event `self.ReceiveBeginPlay`
  (bind _papersprite (`self.PaperSprite`))
  ;[1 1 1] Setup
  (bind _asmy_player_paper_with_camera (cast `/Game/Blueprints/MyPlayerPaperWithCamera` (`GameplayStatics.GetPlayerCharacter` 0)))
  (bind _output_get (set `self.Player` _asmy_player_paper_with_camera))
  (if (== 5 (`KismetMathLibrary.RandomIntegerInRange` 0 5))
    (set `self.CoinValue` 500)
    (`PaperSpriteComponent.SetSprite` _papersprite "/Game/Art/Sprites/Wall_InnerCorner_Sprite.Wall_InnerCorner_Sprite")
    (`PaperSpriteComponent.SetSpriteColor` _papersprite (struct :`R` 0.079982 :`G` 1.0 :`A` 1.0))
    (else
      (set `self.CoinValue` 50)
      (`PaperSpriteComponent.SetSprite` _papersprite "/Game/Art/Sprites/Wall_InnerCorner_Sprite.Wall_InnerCorner_Sprite"))))

(event `self.ReceiveActorBeginOverlap`
  (params (OtherActor :type "Actor Object Reference"))
  ;[1 1 1] Player has collected this
  (if (== OtherActor (`self.Player`))
    (`ScoreSystemComponent.AddScore` (`/Game/Blueprints/MyPlayerPaperWithCamera.ScoreSystem` (stale `self.ReceiveBeginPlay` _output_get)) (`self.CoinValue`))
    (`self.K2_DestroyActor`)))

(event `self.ReceiveTick`
  (params (DeltaSeconds :type "Float (single-precision)"))
  (bind _papersprite (`self.PaperSprite`))
  (bind _papersprite_2 (`self.PaperSprite`))
  (bind _returnvalue (`KismetStringLibrary.Conv_IntToString` (`self.CoinValue`)))
  ;[1 1 1] Change Sprite on runtime
  (if (> (`/Game/Blueprints/MyPlayerPaperWithCamera.SweetSpotComboAmount` (`self.Player`)) 4)
    (set `self.ComboOn` true)
    (switch `string` _returnvalue
      (:`50`
        (`PaperSpriteComponent.SetSprite` _papersprite_2 "/Game/Art/Placeholder/Sprite_1_Sprite_0.Sprite_1_Sprite_0")
        (set `self.CoinValue` 100))
      (:`500`
        (`PaperSpriteComponent.SetSprite` _papersprite_2 "/Game/Art/Placeholder/Sprite_1_Sprite_0.Sprite_1_Sprite_0")
        (set `self.CoinValue` 1000)))
    (elif (`self.ComboOn`)
      (set `self.ComboOn` false)
      (switch `string` _returnvalue
        (:`100`
          (set `self.CoinValue` 50)
          (`PaperSpriteComponent.SetSprite` _papersprite "/Game/Art/Sprites/Wall_InnerCorner_Sprite.Wall_InnerCorner_Sprite"))
        (:`1000`
          (set `self.CoinValue` 500)
          (`PaperSpriteComponent.SetSprite` _papersprite "/Game/Art/Sprites/Wall_InnerCorner_Sprite.Wall_InnerCorner_Sprite")
          (`PaperSpriteComponent.SetSpriteColor` _papersprite (struct :`R` 0.079982 :`G` 1.0 :`A` 1.0)))))))

(fn `UserConstructionScript`)