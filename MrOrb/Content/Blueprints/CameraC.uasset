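; Camera controller for a vertical 2D climber that follows the player's highest point and ends the run when they fall too far below it.
; BeginPlay detaches the player's CameraBoom; Tick raises it with speed-offset interpolation and eases ortho zoom with boost speed.
; Falling out of view shows the Restart widget and disables input; touch reloads the level.
; UpdateParallax sets a background material parameter but is never called here.
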(event `self.ReceiveBeginPlay`
  (bind _outactors (`GameplayStatics.GetAllActorsOfClass` "/Game/Blueprints/MyPlayerPaperWithCamera.MyPlayerPaperWithCamera_C"))
  (for _array_element _outactors
    (set `self.PlayerRef` _array_element)
    (`SceneComponent.K2_DetachFromComponent` (`/Game/Blueprints/MyPlayerPaperWithCamera.CameraBoom` (`self.PlayerRef`)) "KeepWorld" "KeepWorld" "KeepWorld" true)
    (`SceneComponent.K2_SetWorldLocation` (`/Game/Blueprints/MyPlayerPaperWithCamera.CameraBoom` (`self.PlayerRef`)) (`KismetMathLibrary.MakeVector` 0.0 0.0 (+ (`/Game/Blueprints/MyPlayerPaperWithCamera.HighestPoint` (`self.PlayerRef`)) (`self.OffsetZ`) (`self.StartOffset`))) false false)))

(event `self.ReceiveTick`
  (params (DeltaSeconds :type "Float (single-precision)"))
  (bind _playerref (`self.PlayerRef`))
  (bind _playerref_2 (`self.PlayerRef`))
  (set `self.Pressed` (`.bIsCurrentlyPressed` (`PlayerController.GetInputTouchState` (`GameplayStatics.GetPlayerController` 0) "Touch1")))
  (`self.CameraMovement`)
  (`self.Zoom`)
  (if (`self.Dead`)
    (`/Game/Blueprints/MyPlayerPaperWithCamera.StopPlayerMovement` _playerref_2)
    (`self.DisableInput` _playerref_2 (`GameplayStatics.GetPlayerController` 0))
    (if (`self.Pressed`)
      (while (!= (`self.Pressed`) true)
        _)
      (bind _returnvalue (`GameplayStatics.GetCurrentLevelName` true))
      (`GameplayStatics.OpenLevel` (`KismetStringLibrary.Conv_StringToName` _returnvalue))
      (set `/Game/Blueprints/MyPlayerPaperWithCamera.GameStart` false _playerref)
      (set `/Game/Blueprints/MyPlayerPaperWithCamera.Boost` false _playerref))))

(fn `CameraMovement`
  (bind _playerref (`self.PlayerRef`))
  (bind _playerref_2 (`self.PlayerRef`))
  (bind _playerref_3 (`self.PlayerRef`))
  (bind _playerref_4 (`self.PlayerRef`))
  (bind _camera (`/Game/Blueprints/MyPlayerPaperWithCamera.Camera` (`self.PlayerRef`)))
  (bind _output_get (set `/Game/Blueprints/MyPlayerPaperWithCamera.PlayerHeight` (.z (`self.K2_GetActorLocation` (`self.PlayerRef`))) _playerref_2))
  (if (> (`/Game/Blueprints/MyPlayerPaperWithCamera.PlayerHeight` _playerref_3) (`/Game/Blueprints/MyPlayerPaperWithCamera.HighestPoint` _playerref_3))
    (set `/Game/Blueprints/MyPlayerPaperWithCamera.HighestPoint` _output_get _playerref_2)
    (`SceneComponent.K2_SetWorldLocation` (`/Game/Blueprints/MyPlayerPaperWithCamera.CameraBoom` _playerref_2) (`KismetMathLibrary.MakeVector` 0.0 0.0 (`KismetMathLibrary.FInterpTo` (.z (`SceneComponent.K2_GetComponentLocation` (`/Game/Blueprints/MyPlayerPaperWithCamera.CameraBoom` (`self.PlayerRef`)))) (+ (`/Game/Blueprints/MyPlayerPaperWithCamera.HighestPoint` _playerref) (`self.OffsetZ`) (/ (`KismetMathLibrary.Conv_IntToDouble` (`SpeedComponent.CurrentSpeed` (`/Game/Blueprints/MyPlayerPaperWithCamera.Speed` _playerref))) 5.0)) (`GameplayStatics.GetWorldDeltaSeconds`) 7.5)) false false)
    (return)
    (elif (> (/ (+ (- (`/Game/Blueprints/MyPlayerPaperWithCamera.HighestPoint` _playerref_4) (`/Game/Blueprints/MyPlayerPaperWithCamera.PlayerHeight` _playerref_4)) (`self.OffsetZ`)) (/ (`CameraComponent.OrthoWidth` _camera) (`CameraComponent.AspectRatio` _camera))) 1.5)
      (`self.GameOver`))))

(fn `GameOver`
  (`CharacterMovementComponent.DisableMovement` (`Character.CharacterMovement` (`self.PlayerRef`)))
  (bind _returnvalue (`|CreateWidget` "/Game/Blueprints/Restart.Restart_C"))
  (`UserWidget.AddToViewport` _returnvalue 0)
  (set `self.Dead` true)
  (return))

(fn `UpdateParallax`
  (bind _playerref (`self.PlayerRef`))
  (bind _highestpoint (`/Game/Blueprints/MyPlayerPaperWithCamera.HighestPoint` _playerref))
  (if (not (< (`/Game/Blueprints/MyPlayerPaperWithCamera.PlayerHeight` _playerref) _highestpoint))
    (`KismetMaterialLibrary.SetScalarParameterValue` "/Game/Blueprints/Assets/Temp_Collection.Temp_Collection" "BackgroundOffsetY" (`KismetMathLibrary.Lerp` 0.0 1.0 (/ _highestpoint -40000.0)))
    (return)))

(fn `UserConstructionScript`)

(fn `Zoom`
  (if (> (`SpeedComponent.BoostedSpeed` (`/Game/Blueprints/MyPlayerPaperWithCamera.Speed` (`self.PlayerRef`))) 100)
    (`CameraComponent.SetOrthoWidth` (`/Game/Blueprints/MyPlayerPaperWithCamera.Camera` (`self.PlayerRef`)) (`KismetMathLibrary.FInterpTo` (`CameraComponent.OrthoWidth` (`/Game/Blueprints/MyPlayerPaperWithCamera.Camera` (`self.PlayerRef`))) (`self.MaxZoom`) (`GameplayStatics.GetWorldDeltaSeconds`) 2.5))
    (return)
    (else
      (`CameraComponent.SetOrthoWidth` (`/Game/Blueprints/MyPlayerPaperWithCamera.Camera` (`self.PlayerRef`)) (`KismetMathLibrary.FInterpTo` (`CameraComponent.OrthoWidth` (`/Game/Blueprints/MyPlayerPaperWithCamera.Camera` (`self.PlayerRef`))) (`self.MinZoom`) (`GameplayStatics.GetWorldDeltaSeconds`) 0.5))
      (return))))