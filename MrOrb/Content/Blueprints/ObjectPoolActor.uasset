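; Actor that provides an object pool of static mesh components, switching them between hidden and visible for reuse.
; CreateObjectPool adds hidden components with a given mesh to an available array.
; GetFromObjectPool removes the last available entry, but then re-reads the new last one to mark in-use, unhide and return.
; ReturnToObjectPool re-hides and re-appends components; only unconnected test nodes call these functions here.
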(event `self.ReceiveBeginPlay`)

(fn `CreateObjectPool`
  (params (Mesh :type "StaticMesh Object Reference") (Count :type Integer :default 100))
  ;[1 1 1] Create Pool
  (for _ (range (+ Count 1))
    (bind _returnvalue (`AddComponent|NODE_AddStaticMeshComponent-0` :`bManualAttachment` true :`RelativeTransform` (`KismetMathLibrary.MakeTransform` (0.0 0.0 0.0))))
    (`StaticMeshComponent.SetStaticMesh` _returnvalue Mesh)
    (`SceneComponent.SetHiddenInGame` _returnvalue true true)
    (`KismetArrayLibrary.Array_Add` (`self.AvailableStaticMeshComponentPool`) _returnvalue)))

(fn `GetFromObjectPool`
  (returns (MeshForUse :type "StaticMeshComponent Object Reference"))
  (bind _availablestaticmeshcomponentpool (`self.AvailableStaticMeshComponentPool`))
  (bind _returnvalue (- (`KismetArrayLibrary.Array_Length` _availablestaticmeshcomponentpool) 1))
  (bind _output (`|GetArrayItem` _availablestaticmeshcomponentpool _returnvalue))
  ;[1 1 1] Get Mesh From Pool
  (`KismetArrayLibrary.Array_Remove` _availablestaticmeshcomponentpool _returnvalue)
  (`KismetArrayLibrary.Array_Add` (`self.InUseStaticMeshComponentPool`) _output)
  (`SceneComponent.SetHiddenInGame` _output false false)
  (return _output))

(fn `ReturnToObjectPool`
  (params (MeshReturned :type "StaticMeshComponent Object Reference"))
  (bind _availablestaticmeshcomponentpool (`self.AvailableStaticMeshComponentPool`))
  ;[1 1 1] Return Mesh to Pool
  (`SceneComponent.SetHiddenInGame` MeshReturned true true)
  (`KismetArrayLibrary.Array_RemoveItem` (`self.InUseStaticMeshComponentPool`) MeshReturned)
  (`KismetArrayLibrary.Array_Insert` _availablestaticmeshcomponentpool MeshReturned (`KismetArrayLibrary.Array_Length` _availablestaticmeshcomponentpool)))

(fn `UserConstructionScript`)