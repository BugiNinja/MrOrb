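; Player Blueprint that enables input from the first player controller and turns on physics for its Collider when play begins.
; A ChangeGravity function sets physics simulation and gravity on the Collider, but its branch is fixed to true, so the UseGravity argument has no effect.
; Unconnected leftover nodes reference falling movement, camera boom detachment and a collision particle, and never run.
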(event `self.ReceiveBeginPlay`
  (`self.EnableInput` (`GameplayStatics.GetPlayerController` 0))
  (`self.ChangeGravity` true))

(fn `ChangeGravity`
  (params (UseGravity :type Boolean))
  (bind _collider (`self.Collider`))
  (if true
    (`PrimitiveComponent.SetSimulatePhysics` _collider true)
    (`PrimitiveComponent.SetEnableGravity` _collider true)
    (else
      (`PrimitiveComponent.SetSimulatePhysics` _collider false)
      (`PrimitiveComponent.SetEnableGravity` _collider false)))
  (return))

(fn `UserConstructionScript`)