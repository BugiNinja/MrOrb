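; Bumper actor that knocks the player away on contact, in the X-Z plane.
; On hit it sets the player to falling, calls ChangeGravity off and adds a velocity impulse along the negated hit normal, scaled by twice the player's current boosted speed.
; After a short delay it turns gravity back on.
; HitOnce is set during the bounce but never checked, and a StopPlayerMovement call is left unconnected.
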(event `self.ReceiveHit`
  (params (MyComp :type "PrimitiveComponent Object Reference") (Other :type "Actor Object Reference") (OtherComp :type "PrimitiveComponent Object Reference") (bSelfMoved :type Boolean) (HitLocation :type "Vector Structure") (HitNormal :type "Vector Structure") (NormalImpulse :type "Vector Structure") (Hit :type "HitResult Structure (by ref)"))
  (bind _asplayer_bp (cast `/Game/Blueprints/Player_bp` Other))
  (set `self.Hit once` true)
  (`CharacterMovementComponent.SetMovementMode` (`Character.CharacterMovement` _asplayer_bp) "MOVE_Falling" 0)
  (`/Game/Blueprints/Player_bp.ChangeGravity` _asplayer_bp false)
  (`CharacterMovementComponent.AddImpulse` (`Character.CharacterMovement` _asplayer_bp) (* (* (`KismetMathLibrary.MakeVector` (.x HitNormal) 0.0 (.z HitNormal)) -2.0) (`SpeedComponent.CurrentBoostedSpeed` (`/Game/Blueprints/Player_bp.Speed` _asplayer_bp))) true)
  (`KismetSystemLibrary.Delay` 0.2)
  (`/Game/Blueprints/Player_bp.ChangeGravity` _asplayer_bp true)
  (set `self.Hit once` false))

(fn `UserConstructionScript`)