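; Camera controller for a vertical climbing game that detaches the player's camera boom, follows the highest point reached and handles game over.
; Each tick it eases the boom toward that height plus speed-based offsets, widens orthographic zoom during boosts and drives background parallax through a material parameter collection.
; Falling below the screen margin outside start idle marks the player dead, stops movement and shows the Restart widget.
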(event `self.ReceiveBeginPlay`
  (bind _cameraposition (`self.CalculateStartCamera`))
  (bind _playerref (`self.PlayerRef`))
  (bind _outactors (`GameplayStatics.GetAllActorsOfClass` "/Game/Blueprints/Player_bp.Player_bp_C"))
  (for _array_element _outactors
    (bind _output_get (set `self.PlayerRef` _array_element))
    (`SceneComponent.K2_DetachFromComponent` (`/Game/Blueprints/Player_bp.CameraBoom` _output_get) "KeepWorld" "KeepWorld" "KeepWorld" true)
    (set `/Game/Blueprints/Player_bp.cameraStartPos` _cameraposition _playerref)
    (`SceneComponent.K2_SetWorldLocation` (`/Game/Blueprints/Player_bp.CameraBoom` _playerref) _cameraposition false false)
    (bind _outactors_2 (`GameplayStatics.GetAllActorsOfClass` "/Game/Blueprints/Restart_bp.Restart_bp_C"))
    (for _array_element_2 _outactors_2
      (set `self.RestartRef` _array_element_2)
      (bind _returnvalue (`|CreateWidget` "/Game/Blueprints/Restart.Restart_C"))
      (`UserWidget.AddToViewport` _returnvalue 0)
      (bind _output_get_2 (set `self.RestartUI` _returnvalue))
      (`Widget.SetVisibility` _output_get_2 "Hidden"))))

(event `self.ReceiveTick`
  (params (DeltaSeconds :type "Float (single-precision)"))
  (bind _playerref (`self.PlayerRef`))
  (if (`/Game/Blueprints/Player_bp.Dead` _playerref)
    (`/Game/Blueprints/Player_bp.StopPlayerMovement` _playerref)
    (`Widget.SetVisibility` (`self.RestartUI`) "Visible")
    (else
      ;[1 1 1] Basic update
      (`self.UpdateParallax`)
      (`self.CameraMovement`)
      (`self.Zoom`)
      (`Widget.SetVisibility` (`self.RestartUI`) "Hidden"))))

(fn `CameraMovement`
  (bind _playerref (`self.PlayerRef`))
  (bind _playerref_2 (`self.PlayerRef`))
  (if (`self.IsPlayerOutsideCamera`)
    (`self.SetPlayerHeight`)
    (if (`self.IsPlayerAtHighestPoint`)
      (set `/Game/Blueprints/Player_bp.HighestPoint` (`/Game/Blueprints/Player_bp.PlayerHeight` _playerref_2) _playerref_2))
    (`SceneComponent.K2_SetWorldLocation` (`/Game/Blueprints/Player_bp.CameraBoom` _playerref_2) (`self.CalculateNewCameraHeight`) false false)
    (return)
    (elif (not (`/Game/Blueprints/Player_bp.StartIdle` (`self.PlayerRef`)))
      (set `/Game/Blueprints/Player_bp.Dead` true _playerref)
      (`/Game/Blueprints/Player_bp.StopPlayerMovement` _playerref))))

(fn `SetPlayerHeight`
  (bind _playerref (`self.PlayerRef`))
  (set `/Game/Blueprints/Player_bp.PlayerHeight` (.z (`self.K2_GetActorLocation` _playerref)) _playerref)
  (return))

(fn `UpdateParallax`
  (bind _playerref (`self.PlayerRef`))
  (bind _highestpoint (`/Game/Blueprints/Player_bp.HighestPoint` _playerref))
  (if (< (`/Game/Blueprints/Player_bp.PlayerHeight` _playerref) _highestpoint)
    _
    (else
      _))
  (`KismetMaterialLibrary.SetScalarParameterValue` "/Game/Blueprints/Assets/Temp_Collection.Temp_Collection" "BackgroundOffsetY" (`KismetMathLibrary.Lerp` 0.0 1.0 (/ _highestpoint -40000.0)))
  (return))

(fn `UserConstructionScript`)

(fn `Zoom`
  (bind _camera (`/Game/Blueprints/Player_bp.Camera` (`self.PlayerRef`)))
  (if (> (`SpeedComponent.BoostedSpeed` (`/Game/Blueprints/Player_bp.Speed` (`self.PlayerRef`))) 100)
    (`CameraComponent.SetOrthoWidth` _camera (`self.CalculateZoomOut`))
    (else
      (`CameraComponent.SetOrthoWidth` _camera (`self.CalculateZoomIn`))))
  (return))