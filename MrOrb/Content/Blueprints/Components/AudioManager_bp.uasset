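; Audio manager Blueprint that plays 2D sounds unless the game is muted.
; Tick casts the player pawn to Player_bp and copies the Muted flag from its menu UI every frame.
; PlaySound checks that cached flag before playing the sound passed in.
; BeginPlay sets the wall hit and boost sound variables to None, and nothing here plays them.
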(event `self.ReceiveBeginPlay`
  (set `self.WallHitSound` null)
  (set `self.BoostSound` null))

(event `self.ReceiveTick`
  (params (DeltaSeconds :type "Float (single-precision)"))
  (bind _asplayer_bp (cast `/Game/Blueprints/Player_bp` (`GameplayStatics.GetPlayerPawn` 0)))
  (set `self.Muted` (`/Game/Blueprints/UI/Menu.Muted` (`/Game/Blueprints/Player_bp.MenuUIRef` _asplayer_bp))))

(fn `Play Sound`
  (params (Sound :type "SoundCue Object Reference"))
  (if (not (`self.Muted`))
    (`GameplayStatics.PlaySound2D` Sound 1.0 1.0 0.0 null null)))

(fn `UserConstructionScript`)