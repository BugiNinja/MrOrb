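; Level color changer that shifts wall, wall outline, background and parallax colors as the player moves through height-based levels.
; Each tick it derives a level index from the player's Z position divided by LevelLength.
; Four update functions look up that level's colors by constructed parameter name in the LevelColors parameter collection and interpolate the live parameters toward them.
; An older lifebar- and speed-driven color chain remains unconnected.
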(event `self.ReceiveTick`
  (params (DeltaSeconds :type "Float (single-precision)"))
  (set `self.DeltaTime` DeltaSeconds)
  (`self.TrackPlayerLevel`)
  (`self.UpdateWallOutlineColor`)
  (`self.UpdateWallColor`)
  (`self.UpdateBackgroundColor`)
  (`self.UpdateParallaxColor`))

(fn `TrackPlayerLevel`
  ;[1 1 1] Track Player Level
  (set `self.Levelindex` (+ (`KismetMathLibrary.FTrunc` (/ (.z (`self.K2_GetActorLocation` (`GameplayStatics.GetPlayerCharacter` 0))) (`self.LevelLength`))) 1)))

(fn `UpdateBackgroundColor`
  (bind _returnvalue (`KismetStringLibrary.Conv_StringToName` "Background Tint"))
  (bind _returnvalue_2 (`KismetMaterialLibrary.GetVectorParameterValue` "/Game/Art/Materials/LevelColors.LevelColors" (`KismetStringLibrary.Conv_StringToName` (`KismetStringLibrary.Concat_StrStr` "BG" (`KismetStringLibrary.Conv_IntToString` (`self.Levelindex`))))))
  (bind _returnvalue_3 (`KismetMaterialLibrary.GetVectorParameterValue` "/Game/Art/Materials/LevelColors.LevelColors" _returnvalue))
  (`KismetMaterialLibrary.SetVectorParameterValue` "/Game/Art/Materials/LevelColors.LevelColors" _returnvalue (`KismetMathLibrary.CInterpTo` _returnvalue_3 _returnvalue_2 (`self.DeltaTime`) (`self.ColorInterpolationSpeed`))))

(fn `UpdateParallaxColor`
  (bind _returnvalue (`KismetStringLibrary.Conv_StringToName` "Parallax Layer1 Outline"))
  (bind _returnvalue_2 (`KismetMaterialLibrary.GetVectorParameterValue` "/Game/Art/Materials/LevelColors.LevelColors" (`KismetStringLibrary.Conv_StringToName` (`KismetStringLibrary.Concat_StrStr` "BG Parallax" (`KismetStringLibrary.Conv_IntToString` (`self.Levelindex`))))))
  (bind _returnvalue_3 (`KismetMaterialLibrary.GetVectorParameterValue` "/Game/Art/Materials/LevelColors.LevelColors" _returnvalue))
  (`KismetMaterialLibrary.SetVectorParameterValue` "/Game/Art/Materials/LevelColors.LevelColors" _returnvalue (`KismetMathLibrary.CInterpTo` _returnvalue_3 _returnvalue_2 (`self.DeltaTime`) (`self.ColorInterpolationSpeed`))))

(fn `UpdateWallColor`
  (bind _returnvalue (`KismetStringLibrary.Conv_StringToName` "Wall Color Main"))
  (bind _returnvalue_2 (`KismetMaterialLibrary.GetVectorParameterValue` "/Game/Art/Materials/LevelColors.LevelColors" (`KismetStringLibrary.Conv_StringToName` (`KismetStringLibrary.Concat_StrStr` "Wall" (`KismetStringLibrary.Conv_IntToString` (`self.Levelindex`))))))
  (bind _returnvalue_3 (`KismetMaterialLibrary.GetVectorParameterValue` "/Game/Art/Materials/LevelColors.LevelColors" _returnvalue))
  (`KismetMaterialLibrary.SetVectorParameterValue` "/Game/Art/Materials/LevelColors.LevelColors" _returnvalue (`KismetMathLibrary.CInterpTo` _returnvalue_3 _returnvalue_2 (`self.DeltaTime`) (`self.ColorInterpolationSpeed`))))

(fn `UpdateWallOutlineColor`
  (bind _returnvalue (`KismetStringLibrary.Conv_StringToName` "Wall Color Outline"))
  (bind _returnvalue_2 (`KismetMaterialLibrary.GetVectorParameterValue` "/Game/Art/Materials/LevelColors.LevelColors" (`KismetStringLibrary.Conv_StringToName` (`KismetStringLibrary.Concat_StrStr` "Wall Outline" (`KismetStringLibrary.Conv_IntToString` (`self.Levelindex`))))))
  (bind _returnvalue_3 (`KismetMaterialLibrary.GetVectorParameterValue` "/Game/Art/Materials/LevelColors.LevelColors" _returnvalue))
  (`KismetMaterialLibrary.SetVectorParameterValue` "/Game/Art/Materials/LevelColors.LevelColors" _returnvalue (`KismetMathLibrary.CInterpTo` _returnvalue_3 _returnvalue_2 (`self.DeltaTime`) (`self.ColorInterpolationSpeed`))))

(fn `UserConstructionScript`)