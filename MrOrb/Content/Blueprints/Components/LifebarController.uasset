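; Lifebar controller that treats the player's life as a countdown timer and sets the player's Dead flag when it runs out.
; While the player lives, Tick counts down by world delta time, or holds at full lifetime during StartIdle.
; The remaining-life percent drives the Time scalar in the ColorCollection material parameter collection.
; AddTime adds an unclamped amount or restores the full lifetime.
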(event `self.ReceiveBeginPlay`
  (set `self.CurrentTime` (`self.WholeLifetime`)))

(event `self.ReceiveTick`
  (params (DeltaSeconds :type "Float (single-precision)"))
  (bind _time_left_in__ (`self.CalcCurrentPercent`))
  (if (`/Game/Blueprints/Player_bp.Dead` (`self.PlayerRef`))
    _
    (elif (`/Game/Blueprints/Player_bp.StartIdle` (`self.PlayerRef`))
      (set `self.CurrentTime` (`self.WholeLifetime`))
      (`KismetMaterialLibrary.SetScalarParameterValue` "/Game/Art/Materials/ColorCollection.ColorCollection" "Time" 1.0)
      (else
        (`self.GetCurrentTime`)
        (`KismetMaterialLibrary.SetScalarParameterValue` "/Game/Art/Materials/ColorCollection.ColorCollection" "Time" _time_left_in__)
        (if (<= _time_left_in__ 0.0)
          (set `/Game/Blueprints/Player_bp.Dead` true (`self.PlayerRef`)))))))

(fn `AddTime`
  (params (Amount :type "Float (double-precision)") (`GetFullTime?` :type Boolean))
  (if `GetFullTime?`
    (set `self.CurrentTime` (`self.WholeLifetime`))
    (else
      (set `self.CurrentTime` (+ Amount (`self.CurrentTime`)))))
  (return))

(fn `GetCurrentTime`
  (set `self.CurrentTime` (- (`self.CurrentTime`) (`GameplayStatics.GetWorldDeltaSeconds`)))
  (return))

(fn `UserConstructionScript`)