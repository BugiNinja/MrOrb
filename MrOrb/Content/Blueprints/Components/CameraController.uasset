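; Camera controller actor for a vertical climbing game that drives an orthographic camera, parallax and menu/restart widgets.
; Tick switches UI by player state: dead, pre-start idle or playing.
; During play it interpolates the boom toward the highest point plus a speed-based offset, zooms with boost speed, and flags death when the player's projected position falls below the screen margin.
; Background parallax follows highest point through a Material Parameter Collection scalar.
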(event `self.ReceiveBeginPlay`
  (bind _cameraposition (`self.CalculateStartCamera`))
  (set `self.CameraZoom` (`CameraComponent.OrthoWidth` (`self.Camera`)))
  (set `self.CameraStartPos` _cameraposition)
  (`SceneComponent.K2_SetWorldLocation` (`self.CameraBoom`) _cameraposition false false)
  (`self.Create UI `)
  (`PlayerController.SetViewTargetWithBlend` (`GameplayStatics.GetPlayerController` 0) self 0.0 "VTBlend_Linear" 0.0 false))

(event `self.ReceiveTick`
  (params (DeltaSeconds :type "Float (single-precision)"))
  (bind _playerref (`self.PlayerRef`))
  (bind _restartui (`self.RestartUI`))
  (bind _playerref_2 (`self.PlayerRef`))
  (bind _menuui (`self.MenuUI`))
  (if (`/Game/Blueprints/Player_bp.Dead` _playerref)
    ;[1 1 1] Game over
    (`/Game/Blueprints/Player_bp.StopPlayerMovement` _playerref)
    (`Widget.SetVisibility` (`self.RestartUI`) "Visible")
    (elif (`/Game/Blueprints/Player_bp.StartIdle` _playerref)
      ;[1 1 1] Before game start
      (`self.UpdateParallax`)
      (`Widget.SetVisibility` (`self.RestartUI`) "Hidden")
      (`Widget.SetVisibility` _menuui "Visible")
      (if (`/Game/Blueprints/UI/Menu.StoreIsActive` _menuui)
        (set `/Game/Blueprints/Player_bp.StoreIsActive` true _playerref_2)
        (else
          (set `/Game/Blueprints/Player_bp.StoreIsActive` false _playerref_2)))
      (else
        ;[1 1 1] Basic update
        (`self.UpdateParallax`)
        (`self.CameraMovement`)
        (`self.Zoom`)
        (`Widget.SetVisibility` (`self.RestartUI`) "Hidden")
        (`Widget.SetVisibility` (`self.MenuUI`) "Hidden")
        (set `/Game/Blueprints/Player_bp.StoreIsActive` false (`self.PlayerRef`))
        (set `/Game/Blueprints/UI/Restart.ContinueTimer` (`/Game/Blueprints/UI/Restart.TimerStartValue` _restartui) _restartui)))))

(fn `CameraMovement`
  (bind _playerref (`self.PlayerRef`))
  (bind _playerref_2 (`self.PlayerRef`))
  (if (`self.IsPlayerOutsideCamera`)
    (`self.SetPlayerHeight`)
    (if (`self.IsPlayerAtHighestPoint`)
      (set `/Game/Blueprints/Player_bp.HighestPoint` (`/Game/Blueprints/Player_bp.PlayerHeight` _playerref_2) _playerref_2))
    (`SceneComponent.K2_SetWorldLocation` (`self.CameraBoom`) (`self.CalculateNewCameraHeight`) false false)
    (return)
    (elif (not (`/Game/Blueprints/Player_bp.StartIdle` (`self.PlayerRef`)))
      (set `/Game/Blueprints/Player_bp.Dead` true _playerref)
      (`/Game/Blueprints/Player_bp.StopPlayerMovement` _playerref))))

(fn `Create UI `
  (bind _playerref (`self.PlayerRef`))
  (bind _returnvalue (`|CreateWidget` "/Game/Blueprints/UI/Restart.Restart_C"))
  (`UserWidget.AddToViewport` _returnvalue 0)
  (bind _output_get (set `self.RestartUI` _returnvalue))
  (`Widget.SetVisibility` _output_get "Hidden")
  (bind _returnvalue_2 (`|CreateWidget` "/Game/Blueprints/UI/Menu.Menu_C"))
  (bind _output_get_2 (set `self.MenuUI` _returnvalue_2))
  (set `/Game/Blueprints/Player_bp.MenuUIRef` _output_get_2 _playerref)
  (set `/Game/Blueprints/UI/Menu.Player` _playerref _output_get_2)
  (`UserWidget.AddToViewport` _output_get_2 0)
  (return))

(fn `SetPlayerHeight`
  (bind _playerref (`self.PlayerRef`))
  (set `/Game/Blueprints/Player_bp.PlayerHeight` (.z (`self.K2_GetActorLocation` _playerref)) _playerref)
  (return))

(fn `UpdateParallax`
  (bind _playerref (`self.PlayerRef`))
  (bind _highestpoint (`/Game/Blueprints/Player_bp.HighestPoint` _playerref))
  (if (< (`/Game/Blueprints/Player_bp.PlayerHeight` _playerref) _highestpoint)
    _
    (else
      _))
  (`KismetMaterialLibrary.SetScalarParameterValue` "/Game/Blueprints/Assets/Temp_Collection.Temp_Collection" "BackgroundOffsetY" (`KismetMathLibrary.Lerp` 0.0 1.0 (/ _highestpoint -40000.0)))
  (return))

(fn `UserConstructionScript`)

(fn `Zoom`
  (bind _camera (`self.Camera`))
  (if (> (`SpeedComponent.BoostedSpeed` (`/Game/Blueprints/Player_bp.Speed` (`self.PlayerRef`))) 100)
    (`CameraComponent.SetOrthoWidth` _camera (`self.CalculateZoomOut`))
    (else
      (`CameraComponent.SetOrthoWidth` _camera (`self.CalculateZoomIn`))))
  (return))