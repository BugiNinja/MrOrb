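; SquareBumper is a bumper that knocks the player away on hit, with the impulse confined to the XZ plane.
; On a Player_bp hit, StopPlayerMovement halts the player, sets Falling mode and calls ChangeGravity(false).
; A velocity-change impulse derived from the hit normal, biased in Z and scaled by the player's base speed, follows with a collision particle burst.
; After a short delay, ChangeGravity(true) runs and HitOnce clears.
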(event `self.ReceiveHit`
  (params (MyComp :type "PrimitiveComponent Object Reference") (Other :type "Actor Object Reference") (OtherComp :type "PrimitiveComponent Object Reference") (bSelfMoved :type Boolean) (HitLocation :type "Vector Structure") (HitNormal :type "Vector Structure") (NormalImpulse :type "Vector Structure") (Hit :type "HitResult Structure (by ref)"))
  (bind _asplayer_bp (cast `/Game/Blueprints/Player_bp` Other))
  (set `self.Hit once` true)
  (bind _playerout (`self.StopPlayerMovement` _asplayer_bp))
  (`CharacterMovementComponent.AddImpulse` (`Character.CharacterMovement` _playerout) (* (* (`KismetMathLibrary.MakeVector` (.x HitNormal) 0.0 (+ (.z HitNormal) -0.5)) -2.0) (`SpeedComponent.BaseSpeed` (`/Game/Blueprints/Player_bp.Speed` _asplayer_bp))) true)
  (`GameplayStatics.SpawnEmitterAtLocation` "/Game/Art/ParticleSystems/P_BumperCollision.P_BumperCollision" HitLocation (`KismetMathLibrary.Conv_VectorToRotator` HitNormal) (3.0 3.0 3.0) true "AutoRelease")
  (`KismetSystemLibrary.Delay` 0.1)
  (`/Game/Blueprints/Player_bp.ChangeGravity` _playerout true)
  (set `self.Hit once` false))

(fn `StopPlayerMovement`
  (params (PlayerBp :type "/Game/Blueprints/Player_bp Object Reference"))
  (returns (PlayerOut :type "/Game/Blueprints/Player_bp Object Reference"))
  (if (`self.Hit once`)
    (`/Game/Blueprints/Player_bp.StopPlayerMovement` PlayerBp)
    (`CharacterMovementComponent.SetMovementMode` (`Character.CharacterMovement` PlayerBp) "MOVE_Falling" 0)
    (`/Game/Blueprints/Player_bp.ChangeGravity` PlayerBp false)
    (return PlayerBp)))

(fn `UserConstructionScript`)