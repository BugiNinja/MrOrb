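; Actor that acts as the player's particle trail, snapping to the Player_bp location every tick and orienting to its movement.
; Pitch is derived from player velocity, then negated or offset by 180 degrees by X/Z direction, with up-left forced to zero rotation.
; Each tick also sets trail scale from CalculateSpeedScale, though the boost-based vector math in that graph is left unconnected.
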(event `self.ReceiveBeginPlay`
  ;[1 1 1] Start
  (bind _outactors (`GameplayStatics.GetAllActorsOfClass` "/Game/Blueprints/Player_bp.Player_bp_C"))
  (for _array_element _outactors
    (set `self.Player` _array_element)))

(event `self.ReceiveTick`
  (params (DeltaSeconds :type "Float (single-precision)"))
  ;[1 1 1] Update
  (`SceneComponent.SetWorldScale3D` (`self.Player_Trail`) (`self.CalculateSpeedScale`))
  (`self.GetBools`)
  (`self.K2_SetActorLocation` (`self.K2_GetActorLocation` (`self.Player`)))
  (`self.Rotate`))

(fn `GetBools`
  (set `self.GoingLeft` (< (.x (`self.GetVelocity` (`self.Player`))) 0.0))
  (set `self.GoingUp` (>= (.z (`self.GetVelocity` (`self.Player`))) 0.0))
  (return))

(fn `GetWantedPitchRot`
  (returns (WantedRot :type "Rotator Structure"))
  (return (`KismetMathLibrary.MakeRotator` 0.0 (.pitch (`KismetMathLibrary.MakeRotFromY` (`self.GetVelocity` (`self.Player`)))))))

(fn `Rotate`
  (bind _goingleft (`self.GoingLeft`))
  (bind _wantedrot (`self.GetWantedPitchRot`))
  (bind _output_get (set `self.WantedRot` _wantedrot))
  (if (`self.GoingUp`)
    (if _goingleft
      (`self.K2_SetActorRotation` (struct))
      (else
        (`self.K2_SetActorRotation` (* _output_get -1))))
    (elif _goingleft
      (bind _returnvalue (`KismetMathLibrary.MakeRotator` 0.0 (+ (.pitch _output_get) 180.0)))
      (`self.K2_SetActorRotation` (* _returnvalue -1))
      (else
        (`self.K2_SetActorRotation` _returnvalue))))
  (return))

(fn `UserConstructionScript`)