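; Tutorial actor that shows a three-page tutorial with touch controls for cycling between pages.
; Tick shows the page matching the Show index and hides the other two.
; Touching either of two sprites steps the index forward or back, wrapping at the ends.
; Releasing Touch1 clears the Tutorial flag on Player_bp, which Tick checks to destroy the actor.
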(event `self.ReceiveBeginPlay`
  (bind _asplayer_bp (cast `/Game/Blueprints/Player_bp` (`GameplayStatics.GetPlayerPawn` 0)))
  (set `self.Player` _asplayer_bp))

(event `self.ReceiveTick`
  (params (DeltaSeconds :type "Float (single-precision)"))
  (bind _1st (`self.1st`))
  (bind _2nd (`self.2nd`))
  (switch `int` (`self.Show`)
    (:`0`
      (`SceneComponent.SetVisibility` _1st true true)
      (`SceneComponent.SetVisibility` _2nd false true)
      (`SceneComponent.SetVisibility` (`self.3rd`) false true))
    (:`1`
      (`SceneComponent.SetVisibility` _2nd true true)
      (`SceneComponent.SetVisibility` _1st false true)
      (`SceneComponent.SetVisibility` (`self.3rd`) false true))
    (:`2`
      (`SceneComponent.SetVisibility` (`self.3rd`) true true)
      (`SceneComponent.SetVisibility` _1st false true)
      (`SceneComponent.SetVisibility` _2nd false true)))
  (if (not (`/Game/Blueprints/Player_bp.Tutorial` (`self.Player`)))
    (`self.K2_DestroyActor`)))

(event `self.TutorialSheet2_Sprite_6.OnInputTouchBegin`
  (params (FingerIndex :type "ETouchIndex Enum" :default "Touch1") (TouchedComponent :type "PrimitiveComponent Object Reference"))
  (bind _output_get (set `self.Show` (+ (`self.Show`) 1)))
  (if (== _output_get 3)
    (set `self.Show` 0)))

(event `self.TutorialSheet2_Sprite_61.OnInputTouchBegin`
  (params (FingerIndex :type "ETouchIndex Enum" :default "Touch1") (TouchedComponent :type "PrimitiveComponent Object Reference"))
  (bind _output_get (set `self.Show` (+ (`self.Show`) -1)))
  (if (== _output_get -1)
    (set `self.Show` 2)))

(event `Key|Touch1`
  (params (Key :type "Key Structure"))
  (:`Released`
    (set `/Game/Blueprints/Player_bp.Tutorial` false (`self.Player`))))

(fn `UserConstructionScript`)