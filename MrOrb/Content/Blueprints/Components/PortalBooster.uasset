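; Booster trigger that launches the player along its pitched up axis, once per overlap until exit.
; On entry it stops movement, switches to falling, changes gravity and adds capsule velocity scaled from base speed and clamped vertical velocity.
; The launch pitch gets a small random offset signed by horizontal travel direction.
; It also calls the player's combo, speed-stage and boost logic and plays a sound.
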(event `self.Box.OnComponentEndOverlap`
  (params (OverlappedComponent :type "PrimitiveComponent Object Reference") (OtherActor :type "Actor Object Reference") (OtherComp :type "PrimitiveComponent Object Reference") (OtherBodyIndex :type Integer))
  (set `self.Hit once` false))

(event `self.Box.OnComponentBeginOverlap`
  (params (OverlappedComponent :type "PrimitiveComponent Object Reference") (OtherActor :type "Actor Object Reference") (OtherComp :type "PrimitiveComponent Object Reference") (OtherBodyIndex :type Integer) (bFromSweep :type Boolean) (SweepResult :type "HitResult Structure (by ref)"))
  (bind _returnvalue (`self.GetVelocity` (`GameplayStatics.GetPlayerCharacter` 0)))
  (bind _asplayer_bp (cast `/Game/Blueprints/Player_bp` OtherActor))
  (if (not (`self.Hit once`))
    (set `self.Hit once` true)
    (`/Game/Blueprints/Player_bp.ComboInfo` _asplayer_bp)
    (bind _adjustedrotation (`self.AdjustRotation` (`self.K2_GetActorRotation`) _returnvalue))
    (bind _playerout (`self.StopPlayerMovement` _asplayer_bp))
    (set `/Game/Blueprints/Player_bp.OnWall` true _playerout)
    (`PrimitiveComponent.SetPhysicsLinearVelocity` (`Character.CapsuleComponent` _playerout) (`KismetMathLibrary.GreaterGreater_VectorRotator` (`KismetMathLibrary.MakeVector` 0.0 0.0 (+ (`KismetMathLibrary.FClamp` (/ (.z _returnvalue) 2.0) 0.0 2000.0) (* (`KismetMathLibrary.Conv_IntToDouble` (`SpeedComponent.BaseSpeed` (`/Game/Blueprints/Player_bp.Speed` _asplayer_bp))) 2.5))) _adjustedrotation) true "None")
    (bind _speed (`/Game/Blueprints/Player_bp.Speed` _playerout))
    (`SpeedComponent.AddSpeedInStages` _speed 1)
    (`SpeedComponent.Boost` _speed 0 0.2 1.0 0.1)
    (`/Game/Blueprints/Components/AudioManager_bp.Play Sound` (`/Game/Blueprints/Player_bp.AudioManager` _playerout) "/Game/Audios/ArrowBoostCue2.ArrowBoostCue2")))

(fn `AdjustRotation`
  (params (BoosterRotation :type "Rotator Structure") (PlayerVelocity :type "Vector Structure"))
  (returns (AdjustedRotation :type "Rotator Structure"))
  (locals (AdjustedRotator :type "Rotator Structure"))
  (bind _pitch (.pitch BoosterRotation))
  (bind _returnvalue (`KismetMathLibrary.Lerp` 2.0 4.0 (`KismetMathLibrary.RandomFloat`)))
  (if (< (.x PlayerVelocity) 0.0)
    (set `local.AdjustedRotator` (`KismetMathLibrary.MakeRotator` 0.0 (+ _pitch (* _returnvalue 1.0))))
    (else
      (set `local.AdjustedRotator` (`KismetMathLibrary.MakeRotator` 0.0 (+ _pitch (* _returnvalue -1.0))))))
  (return (`local.AdjustedRotator`)))

(fn `StopPlayerMovement`
  (params (PlayerBp :type "/Game/Blueprints/Player_bp Object Reference"))
  (returns (PlayerOut :type "/Game/Blueprints/Player_bp Object Reference"))
  (if (`self.Hit once`)
    (`/Game/Blueprints/Player_bp.StopPlayerMovement` PlayerBp)
    (`CharacterMovementComponent.SetMovementMode` (`Character.CharacterMovement` PlayerBp) "MOVE_Falling" 0)
    (`/Game/Blueprints/Player_bp.ChangeGravity` PlayerBp true)
    (return PlayerBp)))

(fn `UserConstructionScript`)