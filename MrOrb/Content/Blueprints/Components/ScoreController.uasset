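; ScoreController manages score UI, combo color feedback and high score saving for the player.
; On BeginPlay it creates the score, actual score and big score widgets, hiding the latter two.
; Tick polls the player's ScoreSystem sweet spot combo, switching a collectible color in a Material Parameter Collection once per threshold crossing.
; App termination or backgrounding tells the ScoreSystem to save high scores.
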(event `self.ReceiveBeginPlay`
  (bind _asplayer_bp (cast `/Game/Blueprints/Player_bp` (`GameplayStatics.GetPlayerCharacter` 0)))
  (set `self.Player` _asplayer_bp)
  (bind _returnvalue (`|CreateWidget` "/Game/Blueprints/UI/ScoreUI.ScoreUI_C"))
  (bind _output_get (set `self.ScoreUIWidget` _returnvalue))
  (bind _returnvalue_2 (`|CreateWidget` "/Game/Blueprints/UI/ActualScoreWidget.ActualScoreWidget_C"))
  (bind _output_get_2 (set `self.ActualScoreWidget` _returnvalue_2))
  (`UserWidget.AddToViewport` _output_get 0)
  (`UserWidget.AddToViewport` _output_get_2 0)
  (`Widget.SetVisibility` _output_get_2 "Hidden")
  (bind _returnvalue_3 (`|CreateWidget` "/Game/Blueprints/UI/BigScoreWidget.BigScoreWidget_C"))
  (bind _output_get_3 (set `self.BigScoreWidget` _returnvalue_3))
  (`UserWidget.AddToViewport` _output_get_3 0)
  (`Widget.SetVisibility` _output_get_3 "Hidden"))

(event `self.ReceiveTick`
  (params (DeltaSeconds :type "Float (single-precision)"))
  (bind _doonce (`self.DoOnce`))
  (bind _returnvalue (`ScoreSystemComponent.GetSweetSpotComboAmount` (`/Game/Blueprints/Player_bp.ScoreSystem` (`self.Player`))))
  (if (>= _returnvalue 5)
    (if _doonce
      (`KismetMaterialLibrary.SetVectorParameterValue` "/Game/Art/Materials/ColorCollection.ColorCollection" "Collectible 1" (`KismetMathLibrary.MakeColor` 90.0 10.0 20.0))
      (set `self.DoOnce` false))
    (elif (not _doonce)
      (`KismetMaterialLibrary.SetVectorParameterValue` "/Game/Art/Materials/ColorCollection.ColorCollection" "Collectible 1" (`KismetMathLibrary.MakeColor` 50.0 29.32))
      (set `self.DoOnce` true))))

(event `self.ApplicationLifecycle.ApplicationWillTerminateDelegate`
  ;[1 1 1] Save Game on Exit
  (`ScoreSystemComponent.SaveHighScoresToMemory` (`/Game/Blueprints/Player_bp.ScoreSystem` (`self.Player`)) :!label _label))

(event `self.ApplicationLifecycle.ApplicationWillEnterBackgroundDelegate`
  ;[1 1 1] Save Game on Exit
  (goto _label))

(fn `UserConstructionScript`)