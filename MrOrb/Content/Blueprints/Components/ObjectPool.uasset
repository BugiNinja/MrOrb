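; Object pool actor that pre-spawns block actors in two groups, 2000 and 3000 height, for reuse.
; On BeginPlay it spawns each listed class hidden at its own transform into an Available array per group.
; TakeObjectFromPool and ReturnObjectToPool move objects between Available and InUse arrays by group flag.
; Take re-rolls its random index at each step, so it can affect different objects; Return unhides rather than hides.
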(event `self.ReceiveBeginPlay`
  (`self.CreatePools` (`self.Blocks2000Height`) (`self.Blocks3000Height`)))

(fn `CreatePools`
  (params (Objects2000 :type "Array of Actor Class Reference") (Objects3000 :type "Array of Actor Class Reference"))
  (for _array_element Objects2000
    (bind _returnvalue (`|SpawnActorFromClass` _array_element (`self.GetTransform`) "AlwaysSpawn" "OverrideRootScale" null null))
    (`self.SetActorHiddenInGame` _returnvalue true)
    (`KismetArrayLibrary.Array_Add` (`self.AvailableObjects2000`) _returnvalue))
  (for _array_element_2 Objects3000
    (bind _returnvalue_2 (`|SpawnActorFromClass` _array_element_2 (`self.GetTransform`) "AlwaysSpawn" "OverrideRootScale" null null))
    (`self.SetActorHiddenInGame` _returnvalue_2 true)
    (`KismetArrayLibrary.Array_Add` (`self.AvailableObjects3000`) _returnvalue_2))
  (return))

(fn `Debug`
  (params (Object :type "Actor Object Reference"))
  (`KismetSystemLibrary.PrintString` (`KismetSystemLibrary.GetDisplayName` Object))
  (`self.K2_SetActorLocation` (+ (`self.K2_GetActorLocation`) (3500.0 0.0 0.0)))
  (return))

(fn `ReturnObjectToPool`
  (params (`2000 ?` :type Boolean) (Object :type "Actor Object Reference"))
  (bind _inuseobjects2000 (`self.InUseObjects2000`))
  (bind _inuseobjects3000 (`self.InUseObjects3000`))
  (if `2000 ?`
    (`KismetArrayLibrary.Array_Remove` _inuseobjects2000 (`KismetArrayLibrary.Array_Find` _inuseobjects2000 Object))
    (`KismetArrayLibrary.Array_Add` (`self.AvailableObjects2000`) Object)
    (`self.SetActorHiddenInGame` Object false)
    (return)
    (else
      (`KismetArrayLibrary.Array_Remove` _inuseobjects3000 (`KismetArrayLibrary.Array_Find` _inuseobjects3000 Object))
      (`KismetArrayLibrary.Array_Add` (`self.AvailableObjects3000`) Object)
      (`self.SetActorHiddenInGame` Object false)
      (return))))

(fn `TakeObjectFromPool`
  (params (`2000 ?` :type Boolean))
  (bind _availableobjects2000 (`self.AvailableObjects2000`))
  (bind _availableobjects3000 (`self.AvailableObjects3000`))
  (bind _returnvalue (`KismetMathLibrary.RandomInteger` (- (`KismetArrayLibrary.Array_Length` _availableobjects2000) 1)))
  (bind _returnvalue_2 (`KismetMathLibrary.RandomInteger` (- (`KismetArrayLibrary.Array_Length` _availableobjects3000) 1)))
  (bind _output (`|GetArrayItem` _availableobjects2000 _returnvalue))
  (bind _output_2 (`|GetArrayItem` _availableobjects3000 _returnvalue_2))
  (if `2000 ?`
    (`KismetArrayLibrary.Array_Remove` (`self.AvailableObjects2000`) _returnvalue)
    (`KismetArrayLibrary.Array_Add` (`self.InUseObjects2000`) _output)
    (`self.SetActorHiddenInGame` _output false)
    (return)
    (else
      (`KismetArrayLibrary.Array_Remove` (`self.AvailableObjects3000`) _returnvalue_2)
      (`KismetArrayLibrary.Array_Add` (`self.InUseObjects3000`) _output_2)
      (`self.SetActorHiddenInGame` _output_2 false)
      (return))))

(fn `UserConstructionScript`)