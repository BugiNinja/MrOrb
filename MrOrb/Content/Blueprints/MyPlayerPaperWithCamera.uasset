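; Player character for a touch-controlled 2D wall-bouncing game, launched off walls by swipes in the X-Z plane.
; Capsule hits on non-Bumper actors open a timed window where a released swipe becomes an impulse, toggling between physics and character movement.
; A sweet-spot timer on release decides whether the Speed component gains stages and ScoreSystem awards combo points, or both streaks reset.
; Tick also applies boost force, drives global slow motion and draws swipe debug shapes.
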(event `self.ReceiveBeginPlay`
  (bind _speed (`self.Speed`))
  ;[1 1 1] Start
  (`self.EnableInput` (`GameplayStatics.GetPlayerController` 0))
  (`self.ChangeGravity` true)
  (`CharacterMovementComponent.SetMovementMode` (`self.CharacterMovement`) "MOVE_Falling" 0)
  (set `self.WallHitParticle` "/Game/Art/ParticleSystems/P_Collision.P_Collision")
  (set `self.GameStart` true)
  (`SpeedComponent.SetStageAmount` _speed 5)
  (`SpeedComponent.SetStageSpeedAmount` _speed 0.2))

(event `self.ReceiveTick`
  (params (DeltaSeconds :type "Float (single-precision)"))
  (bind _onwalltimer (`self.OnWallTimer`))
  ;[1 1 1] Update
  (`self.Add Boost Force`)
  (`self.DrawInputDebug`)
  (`self.SloMo`)
  (if (and (`self.OnWall`) (or (`self.GameStart`) (< _onwalltimer (`self.BoostTimeFrame`))))
    (set `self.OnWallTimer` (+ DeltaSeconds _onwalltimer))
    (`self.AddBoost`)
    (`KismetSystemLibrary.Delay` 0.3)
    (`self.ChangeGravity` true)
    (else
      (set `self.SweetSpotTimer` (+ DeltaSeconds (`self.SweetSpotTimer`))))))

(event `InputAction|Finger1`
  (params (Key :type "Key Structure"))
  ;[1 1 1] Input
)

(event `Key|Touch1`
  (params (Key :type "Key Structure"))
  (bind (_locationx _locationy _biscurrentlypressed) (`PlayerController.GetInputTouchState` (`GameplayStatics.GetPlayerController` 0) "Touch1"))
  (bind _returnvalue (`KismetMathLibrary.MakeVector2D` _locationx _locationy))
  ;[1 1 1] Input
  (:`Pressed`
    (bind _output_get (set `self.TouchStartPos` _returnvalue))
    (`self.StartInputDebug` _output_get (struct :`R` 1.0 :`G` 0.008376 :`A` 1.0) 1.0))
  (:`Released`
    (if (not _biscurrentlypressed)
      (set `self.TouchEndPos` _returnvalue)
      (`self.EndInputDebug`)
      (set `self.Boost` true)
      (set `self.SweetSpotTimer` 0.0))))

(event `self.CapsuleComponent.OnComponentHit`
  (params (HitComponent :type "PrimitiveComponent Object Reference") (OtherActor :type "Actor Object Reference") (OtherComp :type "PrimitiveComponent Object Reference") (NormalImpulse :type "Vector Structure") (Hit :type "HitResult Structure (by ref)"))
  ;[1 1 1] Player hit wall
  (cast `/Game/Blueprints/Bumper` OtherActor
    (:`CastFailed`
      (set `self.LastHitWall` Hit)
      (`self.ChangeGravity` true)
      (if (not (== (`self.LastHit`) OtherActor))
        (set `self.LastHit` OtherActor)
        (set `self.OnWall` true)
        (set `self.OnWallTimer` 0.0)))))

(fn `Add Boost Force`
  (bind _speed (`self.Speed`))
  (bind _capsulecomponent (`self.CapsuleComponent`))
  (bind (_x _y) (`KismetMathLibrary.BreakVector2D` (* (`self.TouchInputNormalized`) (`KismetMathLibrary.Conv_IntToDouble` (`SpeedComponent.BoostedSpeed` _speed)))))
  (if (and (`SceneComponent.IsSimulatingPhysics` _capsulecomponent "None") (< 0.0 (`SpeedComponent.boostTime` _speed)))
    (`PrimitiveComponent.AddForce` _capsulecomponent (`KismetMathLibrary.MakeVector` (* -1.0 _x) 0.0 _y) "None" true)
    (return)
    (else
      (return))))

(fn `AddBoost`
  (bind _speed (`self.Speed`))
  (if (`self.Boost`)
    (set `self.Boost` false)
    (set `self.OnWall` false)
    (set `self.GameStart` false)
    (`self.StopPlayerMovement`)
    (`CharacterMovementComponent.SetMovementMode` (`self.CharacterMovement`) "MOVE_Falling" 0)
    (`self.ChangeGravity` false)
    (if (< (`self.SweetSpotTimer`) (`KismetMathLibrary.Conv_BoolToDouble` (< (`self.SweetSpotTimer`) (/ (`self.SweetSpot`) (* (`SpeedComponent.Stage` _speed) (`SpeedComponent.StageMult` _speed))))))
      (`self.ComboInfo`)
      (`SpeedComponent.AddSpeedInStages` _speed 1)
      (`SpeedComponent.AddSpeed` _speed 50)
      (`SpeedComponent.AddSpeedMult` _speed 0.0)
      (`SpeedComponent.Boost` _speed 0 0.1 1.0 0.1)
      (else
        (set `self.SweetSpotComboAmount` 0)
        (`SpeedComponent.ResetStages` _speed)
        (`SpeedComponent.AddSpeed` _speed 0)
        (`SpeedComponent.AddSpeedMult` _speed 0.0)
        (`SpeedComponent.Boost` _speed 0 0.0 0.0 0.0)))
    (bind _normalizedvector (`self.CalculatePlayerMovement2D`))
    (bind (_x _y) (`KismetMathLibrary.BreakVector2D` _normalizedvector))
    (`CharacterMovementComponent.AddImpulse` (`self.CharacterMovement`) (`KismetMathLibrary.MakeVector` (* -1.0 _x) 0.0 _y) true)
    (`self.SpawnParticle` (`self.LastHitWall`))
    (return)))

(fn `AddSpeed`
  (set `self.2DMultiplier` (+ (`self.2DMultiplier`) 50.0)))

(fn `CalculatePlayerMovement2D`
  (returns (NormalizedVector :type "Vector2D Structure"))
  (bind _touchstartpos (`self.TouchStartPos`))
  (bind _touchendpos (`self.TouchEndPos`))
  (if (or (not (`self.InputBothDir`)) (> (`.Y` (`KismetMathLibrary.BreakVector2D` _touchendpos)) (`.Y` (`KismetMathLibrary.BreakVector2D` _touchstartpos))))
    (set `self.TouchInputNormalized` (`KismetMathLibrary.Normal2D` (- _touchendpos _touchstartpos)))
    (else
      (set `self.TouchInputNormalized` (`KismetMathLibrary.Normal2D` (- _touchstartpos _touchendpos)))))
  (return (* (`self.TouchInputNormalized`) (`KismetMathLibrary.Conv_IntToDouble` (`SpeedComponent.CurrentSpeed` (`self.Speed`))))))

(fn `ChangeGravity`
  (params (UseGravity :type Boolean))
  (if UseGravity
    (`PrimitiveComponent.SetSimulatePhysics` (`self.CapsuleComponent`) true)
    (`PrimitiveComponent.SetEnableGravity` (`self.CapsuleComponent`) true)
    (else
      (`PrimitiveComponent.SetSimulatePhysics` (`self.CapsuleComponent`) false)
      (`PrimitiveComponent.SetEnableGravity` (`self.CapsuleComponent`) false))))

(fn `ComboInfo`
  (bind _sweetspotcomboamount (`self.SweetSpotComboAmount`))
  (bind _scoresystem (`self.ScoreSystem`))
  (set `self.DoingCombo` true)
  (set `self.SweetSpotComboAmount` (+ (`self.SweetSpotComboAmount`) 1))
  (if (>= _sweetspotcomboamount 5)
    (switch `string` (`KismetStringLibrary.Conv_IntToString` _sweetspotcomboamount)
      (:`Default`
        (bind _returnvalue (`SpeedComponent.GetStage` (`self.Speed`) :!label _label))
        (switch `int` _returnvalue
          (:`Default`
            (`ScoreSystemComponent.AddScore` _scoresystem 350))
          (:`0`
            (`ScoreSystemComponent.AddScore` _scoresystem 10 :!label _label_2))
          (:`1`
            (goto _label_2))
          (:`2`
            (`ScoreSystemComponent.AddScore` _scoresystem 40))
          (:`3`
            (`ScoreSystemComponent.AddScore` _scoresystem 100 :!label _label_3))
          (:`4`
            (`ScoreSystemComponent.AddScore` _scoresystem 200))
          (:`5`
            (goto _label_3))))
      (:`5`
        (`ScoreSystemComponent.AddScore` _scoresystem 500))
      (:`10`
        (`ScoreSystemComponent.AddScore` _scoresystem 2000 :!label _label_4))
      (:`20`
        (goto _label_4))
      (:`30`
        (set `self.SweetSpotComboAmount` 10)
        (goto _label_4)))
    (else
      (goto _label)))
  (return))

(fn `DrawInputDebug`
  (if (`self.DrawDebugTouch`)
    (bind _output_get (set `self.DebugLastPos` (`KismetMathLibrary.MakeVector` (.x (`.Location` (`GameplayStatics.BreakHitResult` (`PlayerController.GetHitResultUnderFingerByChannel` (`GameplayStatics.GetPlayerController` 0) "Touch1" "TraceTypeQuery1" true)))) 1.0 (.z (`.Location` (`GameplayStatics.BreakHitResult` (`PlayerController.GetHitResultUnderFingerByChannel` (`GameplayStatics.GetPlayerController` 0) "Touch1" "TraceTypeQuery1" true)))))))
    (`KismetSystemLibrary.DrawDebugLine` (`self.DebugTouchStart`) _output_get (struct :`R` 0.973958 :`A` 1.0) 0.1 0.5)))

(fn `EndInputDebug`
  (bind _debugtouchstart (`self.DebugTouchStart`))
  (set `self.DrawDebugTouch` false)
  (`KismetSystemLibrary.DrawDebugSphere` _debugtouchstart 100.0 12 (struct :`R` 0.112749 :`G` 1.0 :`B` 0.025833 :`A` 1.0) 1.0 1.0)
  (`KismetSystemLibrary.DrawDebugLine` _debugtouchstart (`self.DebugLastPos`) (struct :`R` 0.156324 :`G` 0.973958 :`B` 0.056094 :`A` 1.0) 1.0 1.0))

(fn `SloMo`
  (bind _boostscale (`SpeedComponent.BoostScale` (`self.Speed`)))
  (if (and (`self.OnWall`) (`self.Boost`) (< (`self.OnWallTimer`) (`self.BoostTimeFrame`)))
    (set `self.SlowMo` 0.1)
    (set `self.TimeSpeed` 0.2)
    (else
      (if (or (== 1 (`SpeedComponent.Stage` (`self.Speed`))) (<= 0.9 (`self.SlowMo`)))
        (set `self.SlowMo` 1.0)
        (else
          (set `self.SlowMo` _boostscale)))
      (set `self.TimeSpeed` (+ (/ _boostscale 3.0) (`self.SlowMo`)))))
  (`GameplayStatics.SetGlobalTimeDilation` (`self.TimeSpeed`))
  (return))

(fn `SpawnParticle`
  (params (Hit :type "HitResult Structure"))
  (bind (_bblockinghit _binitialoverlap _time _distance _location) (`GameplayStatics.BreakHitResult` Hit))
  (if (< (.x (`self.K2_GetActorLocation`)) 0.0)
    (`GameplayStatics.SpawnEmitterAtLocation` (`self.WallHitParticle`) _location (struct :`Yaw` 180.0) (-1.0 1.0 1.0) true "ManualRelease")
    (else
      (`GameplayStatics.SpawnEmitterAtLocation` (`self.WallHitParticle`) _location (struct) (1.0 1.0 1.0) true "ManualRelease")))
  (return))

(fn `StartInputDebug`
  (params (Position :type "Vector2D Structure") (Color :type "LinearColor Structure") (Duration :type "Float (double-precision)"))
  (bind _output_get (set `self.DebugTouchStart` (`KismetMathLibrary.MakeVector` (.x (`.Location` (`GameplayStatics.BreakHitResult` (`PlayerController.GetHitResultUnderFingerByChannel` (`GameplayStatics.GetPlayerController` 0) "Touch1" "TraceTypeQuery1" true)))) 1.0 (.z (`.Location` (`GameplayStatics.BreakHitResult` (`PlayerController.GetHitResultUnderFingerByChannel` (`GameplayStatics.GetPlayerController` 0) "Touch1" "TraceTypeQuery1" true)))))))
  (`KismetSystemLibrary.DrawDebugSphere` _output_get 20.0 12 Color Duration 1.0)
  (set `self.DrawDebugTouch` true))

(fn `StopPlayerMovement`
  (`PrimitiveComponent.SetSimulatePhysics` (`self.CapsuleComponent`) false)
  (`PrimitiveComponent.SetEnableGravity` (`self.CapsuleComponent`) false)
  (`PrimitiveComponent.SetAllPhysicsLinearVelocity` (`self.CapsuleComponent`) (0.0 0.0 0.0) false)
  (`CharacterMovementComponent.DisableMovement` (`self.CharacterMovement`)))

(fn `UserConstructionScript`)