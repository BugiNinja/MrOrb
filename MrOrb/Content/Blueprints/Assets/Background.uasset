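; Background actor meant for vertical parallax scrolling against the player's height, though that logic is currently disconnected.
; BeginPlay caches the Player_bp reference and stores the starting Z as an offset.
; The unwired graph derives Z from that offset minus PlayerHeight scaled by ParallaxSpeed, jumping the offset upward to recycle the background once the player climbs far enough above it.
; Tick is empty, so the actor never moves itself.
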(event `self.ReceiveBeginPlay`
  (bind _outactors (`GameplayStatics.GetAllActorsOfClass` "/Game/Blueprints/Player_bp.Player_bp_C"))
  (for _array_element _outactors
    (set `self.Player` _array_element)
    (set `self.OffsetZ` (.z (`self.K2_GetActorLocation`)))))

(event `self.ReceiveTick`
  (params (DeltaSeconds :type "Float (single-precision)")))

(fn `UserConstructionScript`)