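; Background layer actor that scrolls vertically with parallax as the player climbs and recycles itself to stay ahead of them.
; BeginPlay caches the Player_bp actor and the layer's starting Z as an offset.
; Each Tick sets Z to that offset minus PlayerHeight scaled by ParallaxSpeed, with X and Y fixed.
; Once the player rises far enough above the layer, the offset jumps up by a fixed step, repeating the background.
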(event `self.ReceiveBeginPlay`
  (bind _outactors (`GameplayStatics.GetAllActorsOfClass` "/Game/Blueprints/Player_bp.Player_bp_C"))
  (for _array_element _outactors
    (set `self.Player` _array_element)
    (set `self.OffsetZ` (.z (`self.K2_GetActorLocation`)))))

(event `self.ReceiveTick`
  (params (DeltaSeconds :type "Float (single-precision)"))
  (bind _returnvalue (`KismetMathLibrary.MakeVector` 0.0 -1.0 (+ (* (- (.z (`self.K2_GetActorLocation`)) (+ (`/Game/Blueprints/Player_bp.PlayerHeight` (`self.Player`)) (.z (`self.K2_GetActorLocation`)))) (`self.ParallaxSpeed`)) (`self.OffsetZ`))))
  (if (> (`/Game/Blueprints/Player_bp.PlayerHeight` (`self.Player`)) (+ (.z (`self.K2_GetActorLocation`)) 4000.0))
    (set `self.OffsetZ` (+ (`self.OffsetZ`) 12800.0))
    (`self.K2_SetActorRelativeLocation` _returnvalue)
    (else
      (`self.K2_SetActorLocation` _returnvalue))))

(fn `UserConstructionScript`)