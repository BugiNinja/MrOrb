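; Level generator actor that endlessly builds a vertical level by spawning wall blocks ahead of the player as they climb.
; Each Tick compares player height plus a look-ahead against SpawnedBlocks, then spawns a right block and a lower, mirrored left block at fixed X offsets.
; Each side randomly picks NewBlock1 or the rarer NewBlock2, with ObstacleSpawnCooldown blocking consecutive NewBlock2 spawns.
; SpawnedLeft is set but unused by live logic; several leftover nodes are disconnected.
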(event `self.ReceiveTick`
  (params (DeltaSeconds :type "Float (single-precision)"))
  (bind _returnvalue (+ (* (`self.SpawnedBlocks`) 2000.0) -1200.0))
  (bind _returnvalue_2 (`KismetMathLibrary.MakeTransform` (`KismetMathLibrary.MakeVector` 1100.0 0.0 _returnvalue) (struct :`Pitch` 180.0)))
  (bind _returnvalue_3 (`KismetMathLibrary.MakeTransform` (`KismetMathLibrary.MakeVector` -1100.0 0.0 (- _returnvalue 2000.0))))
  ;[1 1 1] When to spawn
  (`/Engine/EditorBlueprintResources/StandardMacros.CompareFloat` (+ (.z (`self.K2_GetActorLocation` (`GameplayStatics.GetPlayerCharacter` 0))) 4000.0) (* (`self.SpawnedBlocks`) 1000.0)
    (:`>`
      (switch `int` (`KismetMathLibrary.RandomIntegerInRange` 0 2)
        (:`0`
          ;[1 1 1] Spawn Right
          (`|SpawnActorFromClass` "/Game/Blueprints/NewBlock1.NewBlock1_C" _returnvalue_2 "AlwaysSpawn" "OverrideRootScale" null null :!label _label)
          (set `self.ObstacleSpawnCooldown` false))
        (:`1`
          (goto _label))
        (:`2`
          (if (`self.ObstacleSpawnCooldown`)
            (goto _label)
            (else
              (`|SpawnActorFromClass` "/Game/Blueprints/NewBlock2.NewBlock2_C" _returnvalue_2 "AlwaysSpawn" "OverrideRootScale" null null)
              (set `self.ObstacleSpawnCooldown` true)))))
      (set `self.SpawnedLeft` false)
      (switch `int` (`KismetMathLibrary.RandomIntegerInRange` 0 2)
        (:`0`
          ;[1 1 1] Spawn Left
          (`|SpawnActorFromClass` "/Game/Blueprints/NewBlock1.NewBlock1_C" _returnvalue_3 "AlwaysSpawn" "OverrideRootScale" null null :!label _label_2)
          (set `self.ObstacleSpawnCooldown` false))
        (:`1`
          (goto _label_2))
        (:`2`
          (if (`self.ObstacleSpawnCooldown`)
            (goto _label_2)
            (else
              (`|SpawnActorFromClass` "/Game/Blueprints/NewBlock2.NewBlock2_C" _returnvalue_3 "AlwaysSpawn" "OverrideRootScale" null null)
              (set `self.ObstacleSpawnCooldown` true)))))
      (set `self.SpawnedLeft` true)
      (set `self.SpawnedBlocks` (+ (`self.SpawnedBlocks`) 0.5)))))

(event `self.ReceiveBeginPlay`)

(fn `UserConstructionScript`)