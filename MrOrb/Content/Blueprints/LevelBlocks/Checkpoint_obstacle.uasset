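; Checkpoint obstacle level block that extends the player's time, shown as a lifebar, when the player overlaps its sprite.
; AddTime adds ExtraTime directly to the lifebar progress bar's percent, capped at full, then the actor destroys itself.
; Tick also destroys it when OutOfScreen returns false, though that function's projected screen-height comparison appears unused.
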(event `self.Sprite.OnComponentBeginOverlap`
  (params (OverlappedComponent :type "PrimitiveComponent Object Reference") (OtherActor :type "Actor Object Reference") (OtherComp :type "PrimitiveComponent Object Reference") (OtherBodyIndex :type Integer) (bFromSweep :type Boolean) (SweepResult :type "HitResult Structure (by ref)"))
  (cast `/Game/Blueprints/Player_bp` OtherActor)
  (`self.AddTime`)
  (`self.K2_DestroyActor`))

(event `self.ReceiveTick`
  (params (DeltaSeconds :type "Float (single-precision)"))
  (if (not (`self.OutOfScreen`))
    (`self.K2_DestroyActor`)))

(event `self.ReceiveBeginPlay`)

(fn `AddTime`
  (bind _progressbar_171 (`/Game/Blueprints/UI/Lifebar.ProgressBar_171` (`/Game/Blueprints/Components/LifebarController.Lifebar` (`self.LifebarContRef`))))
  (bind _returnvalue (+ (`self.ExtraTime`) (`ProgressBar.Percent` _progressbar_171)))
  (if (> _returnvalue 1.0)
    (`ProgressBar.SetPercent` _progressbar_171 1.0)
    (else
      (`ProgressBar.SetPercent` _progressbar_171 _returnvalue))))

(fn `UserConstructionScript`)