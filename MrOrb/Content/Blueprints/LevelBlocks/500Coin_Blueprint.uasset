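; A 500 coin level pickup that the player collects on overlap, with setup, collection and reset delegated to its CoinSystem component.
; BeginPlay hands CoinSystem the player, score system and coin components, then finds the tagged ScoreController.
; On collection it spawns a particle burst and briefly swaps the normal score widget for the big one.
; ResetCoinFunction exposes the coin reset; the distance-based automatic reset is disconnected from Tick.
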(event `self.ReceiveBeginPlay`
  (bind _coinsystem (`self.CoinSystem`))
  ;[1 1 1] Setup
  (bind _asplayer_bp (cast `/Game/Blueprints/Player_bp` (`GameplayStatics.GetPlayerCharacter` 0)))
  (bind _output_get (set `self.Player` _asplayer_bp))
  (`CoinSystem.SetObjects` _coinsystem (`self.DefaultSceneRoot1`) _output_get (`/Game/Blueprints/Player_bp.ScoreSystem` _output_get) (`self.Sprite`) (`self.Glow`) (`self.Box`))
  (`CoinSystem.SetupCoin` _coinsystem)
  (`self.GetScoreController`))

(event `self.ReceiveActorBeginOverlap`
  (params (OtherActor :type "Actor Object Reference"))
  (bind _returnvalue (`self.K2_GetActorLocation`))
  ;[1 1 1] Player has collected this
  (if (== OtherActor (`self.Player`))
    (bind _returnvalue_2 (`CoinSystem.CollidedWithPlayer` (`self.CoinSystem`)))
    (if _returnvalue_2
      (`GameplayStatics.SpawnEmitterAtLocation` "/Game/Art/ParticleSystems/P_Collect.P_Collect" _returnvalue (struct) (1.5 1.5 1.5) true "AutoRelease")
      (set `self.PlayerZ` (.z _returnvalue))
      (`self.UIChange`)
      (`KismetSystemLibrary.Delay` 0.1)
      (`self.ResetUIChange`))))

(event `self.ReceiveTick`
  (params (DeltaSeconds :type "Float (single-precision)")))

(fn `GetScoreController`
  (bind _outactors (`GameplayStatics.GetAllActorsOfClass` "/Game/Blueprints/Components/ScoreController.ScoreController_C"))
  (for _array_element _outactors
    (if (`self.ActorHasTag` _array_element "ScoreController")
      (bind _asscore_controller (cast `/Game/Blueprints/Components/ScoreController` _array_element))
      (set `self.ScoreController` _asscore_controller)
      (return))))

(fn `ResetCoinFunction`
  (`CoinSystem.ResetCoin` (`self.CoinSystem`))
  (return))

(fn `ResetUIChange`
  (bind _scorecontroller (`self.ScoreController`))
  (`Widget.SetVisibility` (`/Game/Blueprints/Components/ScoreController.ActualScoreWidget` _scorecontroller) "Visible")
  (`Widget.SetVisibility` (`/Game/Blueprints/Components/ScoreController.BigScoreWidget` _scorecontroller) "Hidden")
  (return))

(fn `UIChange`
  (bind _scorecontroller (`self.ScoreController`))
  (`Widget.SetVisibility` (`/Game/Blueprints/Components/ScoreController.ActualScoreWidget` _scorecontroller) "Hidden")
  (`Widget.SetVisibility` (`/Game/Blueprints/Components/ScoreController.BigScoreWidget` _scorecontroller) "Visible")
  (return))

(fn `UserConstructionScript`)