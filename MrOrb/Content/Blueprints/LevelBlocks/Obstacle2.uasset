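; Obstacle level block made of three static meshes that stops blocking once the player builds a high enough sweet spot combo.
; BeginPlay caches the Player_bp, and Tick polls its ScoreSystem until the combo reaches the threshold.
; A DoOnce flag then lets the meshes lose collision and switch to a background-layer material a single time.
; ResetBlock restores physics-only collision, the gradient and outline materials, and clears the flag.
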(event `self.ReceiveBeginPlay`
  (bind _asplayer_bp (cast `/Game/Blueprints/Player_bp` (`GameplayStatics.GetPlayerCharacter` 0)))
  (set `self.Player` _asplayer_bp))

(event `self.ReceiveTick`
  (params (DeltaSeconds :type "Float (single-precision)"))
  (bind _staticmesh (`self.StaticMesh`))
  (bind _returnvalue (`ScoreSystemComponent.GetSweetSpotComboAmount` (`/Game/Blueprints/Player_bp.ScoreSystem` (`self.Player`))))
  (if (>= _returnvalue 15)
    (if (not (`self.DoOnce`))
      (`PrimitiveComponent.SetCollisionEnabled` _staticmesh "NoCollision")
      (`PrimitiveComponent.SetCollisionEnabled` (`self.StaticMesh1`) "NoCollision")
      (`PrimitiveComponent.SetCollisionEnabled` (`self.StaticMesh2`) "NoCollision")
      (`PrimitiveComponent.SetMaterial` _staticmesh 0 "/Game/Art/Materials/M_BG_Layer1.M_BG_Layer1")
      (`PrimitiveComponent.SetMaterial` (`self.StaticMesh1`) 0 "/Game/Art/Materials/M_BG_Layer1.M_BG_Layer1")
      (`PrimitiveComponent.SetMaterial` (`self.StaticMesh2`) 0 "/Game/Art/Materials/M_BG_Layer1.M_BG_Layer1")
      (`PrimitiveComponent.SetMaterial` _staticmesh 1 "/Game/Art/Materials/M_BG_Layer1.M_BG_Layer1")
      (`PrimitiveComponent.SetMaterial` (`self.StaticMesh1`) 1 "/Game/Art/Materials/M_BG_Layer1.M_BG_Layer1")
      (`PrimitiveComponent.SetMaterial` (`self.StaticMesh2`) 1 "/Game/Art/Materials/M_BG_Layer1.M_BG_Layer1")
      (set `self.DoOnce` true))))

(fn `ResetBlock`
  (bind _staticmesh (`self.StaticMesh`))
  (`PrimitiveComponent.SetCollisionEnabled` _staticmesh "PhysicsOnly")
  (`PrimitiveComponent.SetCollisionEnabled` (`self.StaticMesh1`) "PhysicsOnly")
  (`PrimitiveComponent.SetCollisionEnabled` (`self.StaticMesh2`) "PhysicsOnly")
  (`PrimitiveComponent.SetMaterial` _staticmesh 0 "/Game/Art/Materials/M_RadialGradient.M_RadialGradient")
  (`PrimitiveComponent.SetMaterial` (`self.StaticMesh1`) 0 "/Game/Art/Materials/M_RadialGradient.M_RadialGradient")
  (`PrimitiveComponent.SetMaterial` (`self.StaticMesh2`) 0 "/Game/Art/Materials/M_RadialGradient.M_RadialGradient")
  (`PrimitiveComponent.SetMaterial` _staticmesh 1 "/Game/Art/Materials/M_Outline.M_Outline")
  (`PrimitiveComponent.SetMaterial` (`self.StaticMesh1`) 1 "/Game/Art/Materials/M_Outline.M_Outline")
  (`PrimitiveComponent.SetMaterial` (`self.StaticMesh2`) 1 "/Game/Art/Materials/M_Outline.M_Outline")
  (set `self.DoOnce` false)
  (return))

(fn `UserConstructionScript`)