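; Checkpoint level block meant to spawn checkpoint obstacles as the player's highest point rises, though its spawning logic is disconnected and never runs.
; That logic repositions the actor relative to the camera and viewport, then converts height into rounded spawn intervals.
; Odd intervals spawn one obstacle, with a Spawned flag reset on even ones.
; SpawObstacle randomizes X placement and passes the Lifebar reference to the new obstacle.
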(event `self.ReceiveTick`
  (params (DeltaSeconds :type "Float (single-precision)")))

(event `self.ReceiveBeginPlay`)

(fn `GetDistance`
  (set `self.Distance` (/ (`/Game/Blueprints/Player_bp.HighestPoint` (`self.PlayerRef`)) (`self.DistanceBetweenSpawns`)))
  (return))

(fn `Spaw Obstacle`
  (bind _returnvalue (`|SpawnActorFromClass` "/Game/Blueprints/LevelBlocks/Checkpoint_obstacle.Checkpoint_obstacle_C" (`KismetMathLibrary.MakeTransform` (`KismetMathLibrary.MakeVector` (+ (.x (.location (`self.GetTransform`))) (`KismetMathLibrary.RandomFloatInRange` -300.0 300.0)) (.y (.location (`self.GetTransform`))) (.z (.location (`self.GetTransform`)))) (.rotation (`self.GetTransform`)) (.scale (`self.GetTransform`))) "AdjustIfPossibleButDontSpawnIfColliding" "OverrideRootScale" null null))
  (set `/Game/Blueprints/LevelBlocks/Checkpoint_obstacle.LifebarContRef` (`self.Lifebar`) _returnvalue))

(fn `UserConstructionScript`)