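; Touch-controlled player character that launches off walls with slingshot-style swipes in the XZ plane.
; Finger press and release give a normalized drag vector, applied reversed as an impulse while on a wall, with gravity toggled off for a short delay.
; Hitting a different actor than last time re-arms the launch and increases its strength.
; Debug spheres mark touches; older cursor-trace and timeline movement logic remains unwired.
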(event `self.ReceiveBeginPlay`
  ;[1 1 1] Start
  (`self.EnableInput` (`GameplayStatics.GetPlayerController` 0))
  (`self.ChangeGravity` true)
  (`CharacterMovementComponent.SetMovementMode` (`self.CharacterMovement`) "MOVE_Falling" 0))

(event `InputTouch`
  (params (Location :type "Vector Structure") (FingerIndex :type "ETouchIndex Enum"))
  ;[1 1 1] Input start
)

(event `Key|Touch1`
  (params (Key :type "Key Structure"))
  ;[1 1 1] Input start
)

(event `self.ReceiveTick`
  (params (DeltaSeconds :type "Float (single-precision)")))

(event `InputTouch`
  (params (Location :type "Vector Structure") (FingerIndex :type "ETouchIndex Enum"))
  ;[1 1 1] Dragging
)

(event `InputTouch`
  (params (Location :type "Vector Structure") (FingerIndex :type "ETouchIndex Enum"))
  ;[1 1 1] Input release
)

(event `Key|Touch1`
  (params (Key :type "Key Structure"))
  ;[1 1 1] Input release
)

(event `InputAction|Finger1`
  (params (Key :type "Key Structure"))
  (bind (_locationx _locationy) (`PlayerController.GetInputTouchState` (`GameplayStatics.GetPlayerController` 0) "Touch1"))
  (bind _returnvalue (`KismetMathLibrary.MakeVector2D` _locationx _locationy))
  (:`Pressed`
    (set `self.TouchStartPos` _returnvalue)
    (`self.DebugTouch` _returnvalue (struct :`G` 1.0 :`B` 0.233816 :`A` 1.0) 2.0))
  (:`Released`
    (set `self.TouchEndPos` _returnvalue)
    (`self.DebugTouch` _returnvalue (struct :`R` 0.703125 :`B` 0.024405 :`A` 1.0) 2.0)
    (if (`self.OnWall`)
      (set `self.OnWall` false)
      (`self.StopPlayerMovement`)
      (`CharacterMovementComponent.SetMovementMode` (`self.CharacterMovement`) "MOVE_Falling" 0)
      (`self.ChangeGravity` false)
      (bind _normalizedvector (`self.CalculatePlayerMovement2D`))
      (bind (_x _y) (`KismetMathLibrary.BreakVector2D` _normalizedvector))
      (`CharacterMovementComponent.AddImpulse` (`self.CharacterMovement`) (`KismetMathLibrary.MakeVector` (* -1.0 _x) 0.0 _y) true)
      (`KismetSystemLibrary.Delay` 0.5)
      (`self.ChangeGravity` true)
      (else
        (set `self.OnWall` false)))))

(event `self.CapsuleComponent.OnComponentHit`
  (params (HitComponent :type "PrimitiveComponent Object Reference") (OtherActor :type "Actor Object Reference") (OtherComp :type "PrimitiveComponent Object Reference") (NormalImpulse :type "Vector Structure") (Hit :type "HitResult Structure (by ref)"))
  (`PrimitiveComponent.SetAllPhysicsLinearVelocity` (`self.CapsuleComponent`) (0.0 0.0 0.0) false)
  (`self.ChangeGravity` true)
  (if (== (`self.LastHit`) OtherActor)
    (`KismetSystemLibrary.PrintString` "Hit same wall twice" true true (struct :`G` 0.66 :`B` 1.0 :`A` 1.0) 0.1)
    (else
      (set `self.LastHit` OtherActor)
      (set `self.OnWall` true)
      (`self.AddSpeed`))))

(fn `AddSpeed`
  (set `self.2DMultiplier` (+ (`self.2DMultiplier`) 50.0)))

(fn `CalculatePlayerMovement2D`
  (returns (NormalizedVector :type "Vector2D Structure"))
  (return (* (`KismetMathLibrary.Normal2D` (- (`self.TouchEndPos`) (`self.TouchStartPos`))) (`self.2DMultiplier`))))

(fn `ChangeGravity`
  (params (UseGravity :type Boolean))
  (if UseGravity
    (`PrimitiveComponent.SetSimulatePhysics` (`self.CapsuleComponent`) true)
    (`PrimitiveComponent.SetEnableGravity` (`self.CapsuleComponent`) true)
    (else
      (`PrimitiveComponent.SetSimulatePhysics` (`self.CapsuleComponent`) false)
      (`PrimitiveComponent.SetEnableGravity` (`self.CapsuleComponent`) false))))

(fn `DebugTouch`
  (params (Position :type "Vector2D Structure") (Color :type "LinearColor Structure") (Duration :type "Float (double-precision)"))
  (bind (_x _y) (`KismetMathLibrary.BreakVector2D` Position))
  (`KismetSystemLibrary.DrawDebugSphere` (`KismetMathLibrary.MakeVector` _x 0.0 (* -1 _y)) 20.0 12 Color Duration 1.0))

(fn `StopPlayerMovement`
  (`PrimitiveComponent.SetSimulatePhysics` (`self.CapsuleComponent`) false)
  (`PrimitiveComponent.SetEnableGravity` (`self.CapsuleComponent`) false)
  (`PrimitiveComponent.SetAllPhysicsLinearVelocity` (`self.CapsuleComponent`) (0.0 0.0 0.0) false)
  (`CharacterMovementComponent.DisableMovement` (`self.CharacterMovement`)))

(fn `UserConstructionScript`)