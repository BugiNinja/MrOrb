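; Player pawn for a touch-controlled 2D game that flings itself from wall to wall in the XZ plane.
; Releasing a drag while on a wall launches it slingshot-style with a CharacterMovement impulse, suspending capsule physics and gravity for half a second.
; Capsule hits zero velocity and restore gravity; hitting a different actor from the last re-arms the launch and increases its strength.
; Debug spheres mark touches; disconnected experimental nodes remain.
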(event `self.ReceiveBeginPlay`
  ;[1 1 1] Start
  (`self.EnableInput` (`GameplayStatics.GetPlayerController` 0))
  (`self.ChangeGravity` true)
  (`CharacterMovementComponent.SetMovementMode` (`self.CharacterMovement`) "MOVE_Falling" 0))

(event `InputTouch`
  (params (Location :type "Vector Structure") (FingerIndex :type "ETouchIndex Enum"))
  ;[1 1 1] Input start
)

(event `Key|Touch1`
  (params (Key :type "Key Structure"))
  ;[1 1 1] Input start
)

(event `InputTouch`
  (params (Location :type "Vector Structure") (FingerIndex :type "ETouchIndex Enum"))
  ;[1 1 1] Dragging
)

(event `InputTouch`
  (params (Location :type "Vector Structure") (FingerIndex :type "ETouchIndex Enum"))
  ;[1 1 1] Input release
)

(event `Key|Touch1`
  (params (Key :type "Key Structure"))
  ;[1 1 1] Input release
)

(event `InputAction|Finger1`
  (params (Key :type "Key Structure")))

(event `Key|Touch1`
  (params (Key :type "Key Structure"))
  (bind (_locationx _locationy _biscurrentlypressed) (`PlayerController.GetInputTouchState` (`GameplayStatics.GetPlayerController` 0) "Touch1"))
  (bind _returnvalue (`KismetMathLibrary.MakeVector2D` _locationx _locationy))
  (:`Pressed`
    (bind _output_get (set `self.TouchStartPos` _returnvalue))
    (`self.DebugTouch` _output_get (struct :`G` 1.0 :`B` 0.233816 :`A` 1.0) 1.0))
  (:`Released`
    (if (not _biscurrentlypressed)
      (bind _output_get_2 (set `self.TouchEndPos` _returnvalue))
      (`self.DebugTouch` _output_get_2 (struct :`R` 0.703125 :`B` 0.024405 :`A` 1.0) 2.0)
      (if (`self.OnWall`)
        (set `self.OnWall` false)
        (`self.StopPlayerMovement`)
        (`CharacterMovementComponent.SetMovementMode` (`self.CharacterMovement`) "MOVE_Falling" 0)
        (`self.ChangeGravity` false)
        (bind _normalizedvector (`self.CalculatePlayerMovement2D`))
        (bind (_x _y) (`KismetMathLibrary.BreakVector2D` _normalizedvector))
        (`CharacterMovementComponent.AddImpulse` (`self.CharacterMovement`) (`KismetMathLibrary.MakeVector` (* -1.0 _x) 0.0 _y) true)
        (`KismetSystemLibrary.Delay` 0.5)
        (`self.ChangeGravity` true)
        (else
          (set `self.OnWall` false))))))

(event `self.ReceiveTick`
  (params (DeltaSeconds :type "Float (single-precision)")))

(event `self.CapsuleComponent.OnComponentHit`
  (params (HitComponent :type "PrimitiveComponent Object Reference") (OtherActor :type "Actor Object Reference") (OtherComp :type "PrimitiveComponent Object Reference") (NormalImpulse :type "Vector Structure") (Hit :type "HitResult Structure (by ref)"))
  (`PrimitiveComponent.SetAllPhysicsLinearVelocity` (`self.CapsuleComponent`) (0.0 0.0 0.0) false)
  (`self.ChangeGravity` true)
  (if (not (== (`self.LastHit`) OtherActor))
    (set `self.LastHit` OtherActor)
    (set `self.OnWall` true)
    (`self.AddSpeed`)))

(fn `AddSpeed`
  (set `self.2DMultiplier` (+ (`self.2DMultiplier`) 50.0)))

(fn `CalculatePlayerMovement2D`
  (returns (NormalizedVector :type "Vector2D Structure"))
  (return (* (`KismetMathLibrary.Normal2D` (- (`self.TouchEndPos`) (`self.TouchStartPos`))) (`self.2DMultiplier`))))

(fn `ChangeGravity`
  (params (UseGravity :type Boolean))
  (if UseGravity
    (`PrimitiveComponent.SetSimulatePhysics` (`self.CapsuleComponent`) true)
    (`PrimitiveComponent.SetEnableGravity` (`self.CapsuleComponent`) true)
    (else
      (`PrimitiveComponent.SetSimulatePhysics` (`self.CapsuleComponent`) false)
      (`PrimitiveComponent.SetEnableGravity` (`self.CapsuleComponent`) false))))

(fn `DebugTouch`
  (params (Position :type "Vector2D Structure") (Color :type "LinearColor Structure") (Duration :type "Float (double-precision)"))
  (`KismetSystemLibrary.DrawDebugSphere` (`.Location` (`GameplayStatics.BreakHitResult` (`PlayerController.GetHitResultUnderFingerByChannel` (`GameplayStatics.GetPlayerController` 0) "Touch1" "TraceTypeQuery1" true))) 20.0 12 Color Duration 1.0))

(fn `StopPlayerMovement`
  (`PrimitiveComponent.SetSimulatePhysics` (`self.CapsuleComponent`) false)
  (`PrimitiveComponent.SetEnableGravity` (`self.CapsuleComponent`) false)
  (`PrimitiveComponent.SetAllPhysicsLinearVelocity` (`self.CapsuleComponent`) (0.0 0.0 0.0) false)
  (`CharacterMovementComponent.DisableMovement` (`self.CharacterMovement`)))

(fn `UserConstructionScript`)